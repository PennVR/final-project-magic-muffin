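; Actor that dissolves its mesh automatically after play begins.
; On BeginPlay it creates a dynamic material instance from slot 0 so the effect applies to this actor alone, then resets Dissolve Amount to zero.
; After a configurable delay, the full dissolve event plays a timeline that drives the Dissolve Amount scalar parameter on that instance.
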(event `self.ReceiveBeginPlay`
  ;[1 1 1] Create Material Instance
  (bind _returnvalue (`PrimitiveComponent.CreateDynamicMaterialInstance` (`self.Mesh`) 0 (`PrimitiveComponent.GetMaterial` (`self.Mesh`) 0))) ; Create an Instanced Material so it can dissolve on this actor alone
  ;[1 1 1] Set Dynamic Material and Apply to Mesh
  (bind _output_get (set `self.Dynamic Material` _returnvalue))
  (`PrimitiveComponent.SetMaterial` (`self.Mesh`) 0 _output_get)
  ;[1 1 1] Force Dissolve Amount to 0
  (`MaterialInstanceDynamic.SetScalarParameterValue` (`self.Dynamic Material`) "Dissolve Amount" 0.0)
  ;[1 1 1] Delay time before Dissolve Event
  (`KismetSystemLibrary.Delay` (`self.Delay_Before_Dissolve`))
  ;[0 0.4461 1] Trigger Dissolve Event
  (`self.Full_Dissolve`))

(event `Full_Dissolve`
  ;[0 0.4385 1] Dissolve Event
  (bind (_direction _dissolve) (`Timeline|Dissolve_Timeline` :!via `PlayFromStart`) ; Over This time, Dissolve Float output to Material Param Input
    (:`Update`
      (`MaterialInstanceDynamic.SetScalarParameterValue` (`self.Dynamic Material`) "Dissolve Amount" _dissolve) ; On Instance Dynamic Material, Dissolve by this amount
    )))

(fn `UserConstructionScript`)